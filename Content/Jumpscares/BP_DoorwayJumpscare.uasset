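; BP_DoorwayJumpscare is a jumpscare actor that slides a mannequin to an end point.
; While its Jumpscare flag is true, Tick moves the Mannequin toward EndPoint's world location at constant Speed using VInterpToConstant, without sweeping.
; The actor destroys itself once the mannequin arrives.
; Nothing in these graphs sets the flag, so the scare relies on it being set elsewhere.
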(event `self.ReceiveTick`
  (params (DeltaSeconds :type "Float (single-precision)"))
  (if (`self.Jumpscare`)
    (`SceneComponent.K2_SetWorldLocation` (`self.Mannequin`) (`KismetMathLibrary.VInterpTo_Constant` (`SceneComponent.K2_GetComponentLocation` (`self.Mannequin`)) (`SceneComponent.K2_GetComponentLocation` (`self.EndPoint`)) DeltaSeconds (`self.Speed`)) false false)
    (if (== (`SceneComponent.K2_GetComponentLocation` (`self.EndPoint`)) (`SceneComponent.K2_GetComponentLocation` (`self.Mannequin`)) :`ErrorTolerance` 0.001)
      (`self.K2_DestroyActor`))))

(fn `UserConstructionScript`)