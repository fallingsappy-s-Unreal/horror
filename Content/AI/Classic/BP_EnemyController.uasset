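; AI controller for classic enemies that runs the BT_Enemy behavior tree on BeginPlay and feeds it player sightings.
; Perception updates for L1_Character actors set the CanSeePlayer blackboard key to match whether the stimulus was sensed.
; A successful sense also sets IsPursuingPlayer, which this controller never clears when the player is lost.
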(event `self.ReceiveBeginPlay`
  (`self.RunBehaviorTree` "/Game/AI/Classic/BT_Enemy.BT_Enemy"))

(event `self.AIPerception.OnTargetPerceptionUpdated`
  (params (Actor :type "Actor Object Reference") (Stimulus :type "AIStimulus Structure"))
  (if (`.bSuccessfullySensed` (break `AIStimulus` Stimulus))
    (cast `/Game/GameBP/Level1/L1_Character` Actor)
    (`BlackboardComponent.SetValueAsBool` (`AIBlueprintHelperLibrary.GetBlackboard` null) "CanSeePlayer" true)
    (`BlackboardComponent.SetValueAsBool` (`AIBlueprintHelperLibrary.GetBlackboard` null) "IsPursuingPlayer" true)
    (else
      (cast `/Game/GameBP/Level1/L1_Character` Actor)
      (`BlackboardComponent.SetValueAsBool` (`AIBlueprintHelperLibrary.GetBlackboard` null) "CanSeePlayer" false))))

(fn `UserConstructionScript`)