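; Inventory component that stores item classes and amounts in a fixed-size slot array, sized from HG_PlayerController at BeginPlay.
; AddItem tops up partial stacks, then fills empty slots, calling itself recursively for overflow and returning any remainder.
; UseItem looks up an actor of the item class, spawning one if none exists, calls its UseItem and removes one from the slot.
; Slot changes refresh the matching inventory grid widget through the player controller.
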(event `self.ReceiveBeginPlay`
  (bind _ashg_player_controller (cast `/Game/GameBP/HG_PlayerController` (`GameplayStatics.GetPlayerController` 0) :!pure true))
  (`KismetArrayLibrary.Array_Resize` (`self.InventorySlots`) (`/Game/GameBP/HG_PlayerController.InventorySlots` _ashg_player_controller))
  (set `self.W_InventoryMenuRef` (`/Game/GameBP/HG_PlayerController.InventoryMenuRef` _ashg_player_controller)))

(fn `AddItem`
  (params (Item :type "/Game/Blueprints/Actors/Inventory/BP_InventoryItem Class Reference") (Amount :type Integer))
  (returns (Success :type Boolean) (Remainder :type Integer))
  (locals (LocalItem :type "/Game/Blueprints/Actors/Inventory/BP_InventoryItem Class Reference") (LocalAmount :type Integer) (LocalMaxStackAmount :type Integer) (LocalIndex :type Integer :default 0))
  (bind (_success _slotindex) (`self.CheckForEmptySlot`))
  (bind (_success_2 _slotindex_2) (`self.CheckForEmptySlot`))
  (bind (_itemdata_itemname _itemdata_icon _itemdata_maxstackamount) (break `/Game/Blueprints/Structs/S_ItemData` (defaults `Object` (`local.LocalItem`))))
  (bind _returnvalue (- (`local.LocalAmount`) 1))
  (set `local.LocalItem` Item)
  (set `local.LocalAmount` Amount)
  (set `local.LocalMaxStackAmount` _itemdata_maxstackamount)
  (if (> _itemdata_maxstackamount 1)
    (bind (_success_3 _index) (`self.CheckForFreeSlot` (`local.LocalItem`)))
    (if _success_3
      (bind _output_get (set `local.LocalIndex` _index))
      (bind _returnvalue_2 (+ (`.Amout` (`self.GetItemDataAtIndex` _output_get)) (`local.LocalAmount`)))
      (if (> _returnvalue_2 (`local.LocalMaxStackAmount`))
        (set `local.LocalAmount` (- _returnvalue_2 (`local.LocalMaxStackAmount`)))
        (`KismetArrayLibrary.Array_Set` (`self.InventorySlots`) (`local.LocalIndex`) (make `/Game/Blueprints/Structs/S_InventoryItem` (`local.LocalItem`) (`local.LocalMaxStackAmount`)))
        (`self.UpdateInventorySlot` (`local.LocalIndex`))
        (bind (_success_4 _remainder) (`self.AddItem` (`local.LocalItem`) (`local.LocalAmount`)))
        (return true _remainder)
        (else
          (`KismetArrayLibrary.Array_Set` (`self.InventorySlots`) (`local.LocalIndex`) (make `/Game/Blueprints/Structs/S_InventoryItem` (`local.LocalItem`) _returnvalue_2))
          (`self.UpdateInventorySlot` (`local.LocalIndex`))
          (return true 0)))
      (elif _success_2
        (set `local.LocalIndex` _slotindex_2)
        (if (> (`local.LocalAmount`) (`local.LocalMaxStackAmount`))
          (`KismetArrayLibrary.Array_Set` (`self.InventorySlots`) (`local.LocalIndex`) (make `/Game/Blueprints/Structs/S_InventoryItem` (`local.LocalItem`) (`local.LocalMaxStackAmount`)))
          (`self.UpdateInventorySlot` (`local.LocalIndex`))
          (bind (_success_5 _remainder_2) (`self.AddItem` (`local.LocalItem`) (- (`local.LocalAmount`) (`local.LocalMaxStackAmount`))))
          (return true _remainder_2)
          (else
            (`KismetArrayLibrary.Array_Set` (`self.InventorySlots`) (`local.LocalIndex`) (make `/Game/Blueprints/Structs/S_InventoryItem` (`local.LocalItem`) (`local.LocalAmount`)))
            (`self.UpdateInventorySlot` (`local.LocalIndex`))
            (return true 0)))
        (else
          (return false (`local.LocalAmount`)))))
    (elif _success
      (set `local.LocalIndex` _slotindex)
      (`KismetArrayLibrary.Array_Set` (`self.InventorySlots`) (`local.LocalIndex`) (make `/Game/Blueprints/Structs/S_InventoryItem` (`local.LocalItem`) 1))
      (`self.UpdateInventorySlot` (`local.LocalIndex`))
      (if (> _returnvalue 0)
        (bind (_success_6 _remainder_3) (`self.AddItem` (`local.LocalItem`) _returnvalue))
        (return true _remainder_3)
        (else
          (return true 0)))
      (else
        (`KismetSystemLibrary.PrintString` "Inventory Is Full")
        (return false (`local.LocalAmount`))))))

(fn `CheckForEmptySlot`
  (returns (Success :type Boolean) (SlotIndex :type Integer))
  (locals (LocalSuccess :type Boolean) (LocalSlotIndex :type Integer))
  (for (_array_element _array_index) (`self.InventorySlots`)
    (if (`KismetSystemLibrary.IsValidClass` (`.InventoryItem_2_693069954DA6581232C529870C158987` (break `/Game/Blueprints/Structs/S_InventoryItem` _array_element)))
      (set `local.LocalSuccess` false)
      (else
        (set `local.LocalSuccess` true)
        (set `local.LocalSlotIndex` _array_index)
        (break))))
  (return (`local.LocalSuccess`) (`local.LocalSlotIndex`)))

(fn `CheckForFreeSlot`
  (params (Item :type "/Game/Blueprints/Actors/Inventory/BP_InventoryItem Class Reference"))
  (returns (Success :type Boolean) (Index :type Integer))
  (locals (LocalSuccess :type Boolean) (LocalIndex :type Integer))
  (bind (_itemdata_itemname _itemdata_icon _itemdata_maxstackamount) (break `/Game/Blueprints/Structs/S_ItemData` (defaults `Object` Item)))
  (for (_array_element _array_index) (`self.InventorySlots`)
    (bind (_inventoryitem _amount) (break `/Game/Blueprints/Structs/S_InventoryItem` _array_element))
    (if (and (== _inventoryitem Item) (< _amount _itemdata_maxstackamount))
      (set `local.LocalSuccess` true)
      (set `local.LocalIndex` _array_index)
      (break)
      (else
        (set `local.LocalSuccess` false))))
  (return (`local.LocalSuccess`) (`local.LocalIndex`)))

(fn `GetItemDataAtIndex`
  (params (Index :type Integer))
  (returns (Item :type "/Game/Blueprints/Actors/Inventory/BP_InventoryItem Class Reference") (Amout :type Integer))
  (bind (_output_inventoryitem _output_amount) (break `/Game/Blueprints/Structs/S_InventoryItem` (`|GetArrayItem` (`self.InventorySlots`) Index)))
  (return _output_inventoryitem _output_amount))

(fn `RemoveItem`
  (params (Index :type Integer))
  (bind (_item _amout) (`self.GetItemDataAtIndex` Index))
  (if (> _amout 1)
    (`KismetArrayLibrary.Array_Set` (`self.InventorySlots`) Index (make `/Game/Blueprints/Structs/S_InventoryItem` _item (- _amout 1)))
    (else
      (`KismetArrayLibrary.Array_Set` (`self.InventorySlots`) Index (make `/Game/Blueprints/Structs/S_InventoryItem` null))))
  (`self.UpdateInventorySlot` Index))

(fn `UpdateInventorySlot`
  (params (Index :type Integer))
  (`/Game/UMG/Inventory/W_InventorySlot.UpdateSlot` (`|GetArrayItem` (`/Game/UMG/Inventory/W_InventoryGrid.Slots` (`/Game/UMG/Inventory/W_InventoryMenu.W_InventoryGrid` (`/Game/GameBP/HG_PlayerController.InventoryMenuRef` (cast `/Game/GameBP/HG_PlayerController` (`GameplayStatics.GetPlayerController` 0) :!pure true)))) Index)))

(fn `UseItem`
  (params (Index :type Integer))
  (locals (LocalIndex :type Integer))
  (bind _output_get (set `local.LocalIndex` Index))
  (bind (_item _amout) (`self.GetItemDataAtIndex` _output_get))
  (if (> _amout 0)
    (bind _returnvalue (`GameplayStatics.GetActorOfClass` _item))
    (`/Engine/EditorBlueprintResources/StandardMacros.IsValid` _returnvalue
      (:`Is Valid`
        _)
      (:`Is Not Valid`
        (`|SpawnActorFromClass` _item (`KismetMathLibrary.MakeTransform` (0.0 0.0 0.0)) "Undefined" "OverrideRootScale" null null)))
    (`/Game/Blueprints/Actors/Inventory/BP_InventoryItem.UseItem` _returnvalue)
    (`self.RemoveItem` (`local.LocalIndex`))
    (`/Game/UMG/Inventory/W_InventoryMenu.CloseDropDownMenu` (`self.W_InventoryMenuRef`))))