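; BP_PickupActor_Note is a note actor that the player examines through an on-screen widget.
; The construction script writes the front and back note text to two text render components.
; BeginPlay caches the first BP_Examination_Note found in the level.
; On the Action input, a failed validity check creates a W_NoteExamination widget with that reference, updates it from this note and adds it to the viewport.
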(event `self.ReceiveBeginPlay`
  (bind _outactors (`GameplayStatics.GetAllActorsOfClass` "/Game/Blueprints/Actors/Inventory/BP_Examination_Note.BP_Examination_Note_C"))
  (set `self.ExaminationRef` (`|GetArrayItem` _outactors)))

(event `InputAction|Action`
  (params (Key :type "Key Structure"))
  (:`Pressed`
    (`/Engine/EditorBlueprintResources/StandardMacros.IsValid` null
      (:`Is Not Valid`
        (bind _returnvalue (`|CreateWidget` "/Game/UMG/W_NoteExamination.W_NoteExamination_C" null (`self.ExaminationRef`)))
        (bind _output_get (set `self.W_ExaminationNote_Ref` _returnvalue))
        (`/Game/UMG/W_NoteExamination.UpdateWidget` _output_get self)
        (`UserWidget.AddToViewport` (`self.W_ExaminationNote_Ref`) 0)))))

(fn `UserConstructionScript`
  (`parent.UserConstructionScript`)
  (`TextRenderComponent.K2_SetText` (`self.FrontTextRender`) (`self.FrontNoteText`))
  (`TextRenderComponent.K2_SetText` (`self.BackTextRenderer`) (`self.BackNoteText`)))