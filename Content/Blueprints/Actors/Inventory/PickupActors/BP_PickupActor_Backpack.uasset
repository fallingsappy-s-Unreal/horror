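; BP_PickupActor_Backpack is a pickup actor that expands the player's inventory capacity.
; When the Action input is pressed, it calls AddMoreSlots on the player's BPCInventory component with its Amount, then destroys itself.
; BeginPlay, overlap and construction only forward to the parent class, and Tick is disabled.
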(event `self.ReceiveBeginPlay`
  (`parent.ReceiveBeginPlay`))

(event `self.ReceiveActorBeginOverlap`
  (params (OtherActor :type "Actor Object Reference"))
  (`parent.ReceiveActorBeginOverlap` OtherActor))

(event `InputAction|Action`
  (params (Key :type "Key Structure"))
  (:`Pressed`
    (`/Game/Blueprints/Components/BPC_Inventory.AddMoreSlots` (`/Game/GameBP/Level1/L1_Character.BPC_Inventory` (`self.PlayerRef`)) (`self.Amount`))
    (`self.K2_DestroyActor`)))

(fn `UserConstructionScript`
  (`parent.UserConstructionScript`))