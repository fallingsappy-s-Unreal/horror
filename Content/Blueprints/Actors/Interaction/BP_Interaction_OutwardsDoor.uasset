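; Interactable swinging door that always opens away from whoever triggers it, whether the player or a BP_Enemy.
; DoorInteract flips the closed state and uses a dot product against the door's forward vector to pick the swing direction, then a timeline lerps the yaw, reversing to close.
; The Box overlap opens and closes it automatically for enemies; any overlap blocks interaction until a closing animation finishes.
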(event `/Game/Blueprints/Interfaces/BPI_Interaction.Interact`
  (if (`self.CanInteract`)
    (`self.DoorInteract` (`self.PlayerRef`) (`self.IsDoorClosed`))))

(event `ToggleDoorOpen`
  (params (IsDoorClosed :type Boolean))
  (if IsDoorClosed
    (bind (_direction _alpha) (`Timeline|OpenDoorTL` :!label _label)
      (:`Update`
        (`SceneComponent.K2_SetRelativeRotation` (`self.Door`) (`KismetMathLibrary.MakeRotator` 0.0 0.0 (`KismetMathLibrary.Lerp` 0.0 (select `bool` (>= (`self.DotProduct`) 0.0) :`false` -90.0 :`true` 90.0) _alpha)) false false))
      (:`Finished`
        (switch `ETimelineDirection` _direction
          (:`Backward`
            (set `self.CanInteract` true)))))
    (else
      (goto _label :!via `ReverseFromEnd`))))

(event `self.Box.OnComponentBeginOverlap`
  (params (OverlappedComponent :type "PrimitiveComponent Object Reference") (OtherActor :type "Actor Object Reference") (OtherComp :type "PrimitiveComponent Object Reference") (OtherBodyIndex :type Integer) (bFromSweep :type Boolean) (SweepResult :type "HitResult Structure (by ref)"))
  (bind _isdoorclosed (`self.IsDoorClosed`))
  (set `self.CanInteract` false)
  (bind _asbp_enemy (cast `/Game/AI/Classic/BP_Enemy` OtherActor))
  (if _isdoorclosed
    (`self.DoorInteract` _asbp_enemy _isdoorclosed)))

(event `self.Box.OnComponentEndOverlap`
  (params (OverlappedComponent :type "PrimitiveComponent Object Reference") (OtherActor :type "Actor Object Reference") (OtherComp :type "PrimitiveComponent Object Reference") (OtherBodyIndex :type Integer))
  (bind _isdoorclosed (`self.IsDoorClosed`))
  (bind _asbp_enemy (cast `/Game/AI/Classic/BP_Enemy` OtherActor))
  (if (not _isdoorclosed)
    (`self.DoorInteract` _asbp_enemy _isdoorclosed)))

(fn `DoorInteract`
  (params (ActorRef :type "Actor Object Reference") (Condition :type Boolean))
  (set `self.LocalIsDoorClosed` Condition)
  (if Condition
    (set `self.IsDoorClosed` false)
    (set `self.DotProduct` (`KismetMathLibrary.Dot_VectorVector` (`KismetMathLibrary.Normal` (- (`self.K2_GetActorLocation` self) (`self.K2_GetActorLocation` ActorRef))) (`self.GetActorForwardVector` self)))
    (else
      (set `self.IsDoorClosed` true)))
  (`self.ToggleDoorOpen` (`self.LocalIsDoorClosed`)))

(fn `UserConstructionScript`
  (`parent.UserConstructionScript`))