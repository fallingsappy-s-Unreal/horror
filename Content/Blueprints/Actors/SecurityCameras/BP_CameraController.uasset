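; Interactable security camera console that lets the player view the level's BP_SecurityCamera actors, gathered at BeginPlay.
; Interacting toggles viewing: it disables character input and look, hides the main HUD, takes input itself and switches the view target to the current camera.
; Space cycles through cameras with wraparound, while Return, Action or a second Interact restores the player's view, HUD and control.
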(event `self.ReceiveBeginPlay`
  (bind _outactors (`GameplayStatics.GetAllActorsOfClass` "/Game/Blueprints/Actors/SecurityCameras/BP_SecurityCamera.BP_SecurityCamera_C"))
  (set `self.SecurityCameras` _outactors))

(event `/Game/Blueprints/Interfaces/BPI_Interaction.Interact`
  (bind _returnvalue (`GameplayStatics.GetPlayerController` 0))
  (if (`self.IsViewingCameras`)
    (`self.LeaveCameraController`)
    (else
      (set `self.IsViewingCameras` true)
      (`self.DisableInput` (`GameplayStatics.GetPlayerCharacter` 0) _returnvalue)
      (`Controller.SetIgnoreLookInput` _returnvalue true)
      (`Widget.SetVisibility` (`/Game/GameBP/Level1/L1_Character.MainHudRef` (cast `/Game/GameBP/Level1/L1_Character` (`GameplayStatics.GetPlayerCharacter` 0) :!pure true)) "Hidden")
      (`self.EnableInput` (`GameplayStatics.GetPlayerController` 0))
      (`self.ViewThroughCamera`))))

(event `LeaveCameraController`
  (bind _returnvalue (`GameplayStatics.GetPlayerController` 0))
  (bind _returnvalue_2 (`GameplayStatics.GetPlayerController` 0))
  (set `self.IsViewingCameras` false)
  (`self.EnableInput` (`GameplayStatics.GetPlayerCharacter` 0) _returnvalue)
  (`Controller.SetIgnoreLookInput` _returnvalue false)
  (`Widget.SetVisibility` (`/Game/GameBP/Level1/L1_Character.MainHudRef` (cast `/Game/GameBP/Level1/L1_Character` (`GameplayStatics.GetPlayerCharacter` 0) :!pure true)) "SelfHitTestInvisible")
  (`self.DisableInput` _returnvalue_2)
  (`PlayerController.SetViewTargetWithBlend` _returnvalue_2 (`GameplayStatics.GetPlayerCharacter` 0) 0.0 "VTBlend_Linear" 0.0 false))

(event `Key|SpaceBar`
  (params (Key :type "Key Structure"))
  (bind _returnvalue (+ (`self.CurrentCameraIndex`) 1))
  (:`Pressed`
    (set `self.CurrentCameraIndex` (select `bool` (> _returnvalue (- (`KismetArrayLibrary.Array_Length` (`self.SecurityCameras`)) 1)) :`false` _returnvalue))
    (`self.ViewThroughCamera`)))

(event `InputAction|Return`
  (params (Key :type "Key Structure"))
  (:`Pressed`
    (`self.LeaveCameraController` :!label _label)))

(event `InputAction|Action`
  (params (Key :type "Key Structure"))
  (:`Pressed`
    (goto _label)))

(fn `UserConstructionScript`)

(fn `ViewThroughCamera`
  (`PlayerController.SetViewTargetWithBlend` (`GameplayStatics.GetPlayerController` 0) (`|GetArrayItem` (`self.SecurityCameras`) (`self.CurrentCameraIndex`)) 0.0 "VTBlend_Linear" 0.0 false)
  (return))