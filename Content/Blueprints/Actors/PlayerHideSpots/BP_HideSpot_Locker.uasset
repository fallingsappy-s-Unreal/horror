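; Locker hide spot for the player, a child Blueprint that adds an animated swinging door to the parent hide spot's interaction.
; Interact locks further interaction and swings the door open with a timeline that lerps its yaw, then calls the parent Interact after a short delay.
; The inherited FinishedMovingED dispatcher triggers a delayed close on a second timeline, which re-enables interaction when it finishes.
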(event `self.ReceiveBeginPlay`
  (`parent.ReceiveBeginPlay`)
  (add `self.FinishedMovingED` (delegate `FinishedMovingED Event`)))

(event `FinishedMovingED Event`
  (`KismetSystemLibrary.Delay` 0.1)
  (`self.CloseDoor`))

(event `/Game/Blueprints/Interfaces/BPI_Interaction.Interact`
  (if (`self.CanInteract`)
    (set `self.CanInteract` false)
    (bind (_direction _alpha) (`Timeline|OpenLockerDoor` :!via `PlayFromStart`)
      (:`Update`
        (`SceneComponent.K2_SetRelativeRotation` (`self.Door`) (`KismetMathLibrary.MakeRotator` 0.0 0.0 (`KismetMathLibrary.Lerp` 0.0 90.0 _alpha)) false false))
      (:`Finished`
        (`KismetSystemLibrary.Delay` 0.1)
        (`parent.Interact`)))))

(event `CloseDoor`
  (bind (_direction _alpha) (`Timeline|CloseLockerDoor` :!via `PlayFromStart`)
    (:`Update`
      (`SceneComponent.K2_SetRelativeRotation` (`self.Door`) (`KismetMathLibrary.MakeRotator` 0.0 0.0 (`KismetMathLibrary.Lerp` 90.0 0.0 _alpha)) false false))
    (:`Finished`
      (set `self.CanInteract` true))))

(fn `UserConstructionScript`
  (`parent.UserConstructionScript`))